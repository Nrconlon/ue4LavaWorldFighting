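; BP_Explosion is a short-lived explosion actor that spawns a particle effect chosen by ExplosionType (small, medium or fireball).
; BeginPlay sets damage, radius and force variables per type, enables and nudges the overlap trigger, fires a radial impulse, then destroys the actor shortly afterwards.
; The trigger's overlap handler is empty: curve-based distance-falloff damage through a hit interface, and a decal spawn, remain as disconnected logic that never runs.
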(event `self.ReceiveBeginPlay`
  (bind _returnvalue (`self.K2_GetActorLocation`))
  (bind _explosion_trigger (`self.Explosion trigger`))
  (switch `|SwitchEnum` (`self.explosion type`)
    (:`Small_Explosion`
      (`GameplayStatics.SpawnEmitterAtLocation` "/Game/Effects/Particle_Systems/P_Explosion_Bomb.P_Explosion_Bomb" _returnvalue)
      (set `self.Explosion damage` 25.0)
      (set `self.Explosion radius` 40.0)
      (set `self.Explosion force` 50.0))
    (:`Medium_Explosion`
      ;[1 1 1] Not used atm
      (`GameplayStatics.SpawnEmitterAtLocation` "/Game/Effects/Particle_Systems/P_Explosion_Small.P_Explosion_Small" _returnvalue)
      (set `self.Explosion damage` 40.0)
      (set `self.Explosion radius` 160.0)
      (set `self.Explosion force` 60.0))
    (:`Fireball_Explosion`
      (`GameplayStatics.SpawnEmitterAtLocation` "/Game/Effects/Particle_Systems/P_Explosion_Fireball.P_Explosion_Fireball" _returnvalue)
      (set `self.Explosion damage` 30.0)
      (set `self.Explosion radius` 140.0)
      (set `self.Explosion force` 40.0)))
  (`PrimitiveComponent.SetCollisionEnabled` _explosion_trigger "QueryOnly")
  (`SceneComponent.K2_AddLocalOffset` _explosion_trigger (0.0 0.0 0.1) false false)
  (`RadialForceComponent.FireImpulse` (`self.RadialForce1`))
  (`KismetSystemLibrary.Delay` 0.2)
  (`self.K2_DestroyActor`))

(event `self.Explosion trigger.OnComponentBeginOverlap`
  (params (OverlappedComponent :type "PrimitiveComponent Object Reference") (OtherActor :type "Actor Object Reference") (OtherComp :type "PrimitiveComponent Object Reference") (OtherBodyIndex :type Integer) (bFromSweep :type Boolean) (SweepResult :type "HitResult Structure (by ref)")))

(fn `UserConstructionScript`)